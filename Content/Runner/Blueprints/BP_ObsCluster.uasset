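; BP_ObsCluster is an obstacle cluster for the runner game that arranges its child BP_Obs actors in a low/high pattern.
; On BeginPlay it collects those child actors into Obstacles, printing their names, then splits the Combination string into characters.
; Each 0 or 1 teleports the matching obstacle by LowOffset or HighOffset plus a running offset, which grows by LowOffset per character.
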(event `self.ReceiveBeginPlay`
  (for (_array_element _array_index) (`self.GetAllChildActors` self false)
    (`KismetSystemLibrary.PrintString` (`KismetSystemLibrary.GetObjectName` _array_element))
    (bind _asbp_obs (cast `/Game/Runner/Blueprints/BP_Obs` _array_element))
    (`KismetArrayLibrary.Array_Insert` (`self.obstacles`) _asbp_obs _array_index))
  (for (_array_element_2 _array_index_2) (`KismetStringLibrary.ParseIntoArray` (`self.combination`))
    (switch `string` _array_element_2
      (:`0`
        (bind _output (`|GetArrayItem` (`self.obstacles`) _array_index_2))
        (`self.K2_AddActorWorldOffset` _output (+ (`self.lowOffset`) (`self.combinedOffset`)) false true))
      (:`1`
        (`self.K2_AddActorWorldOffset` _output (+ (`self.highOffset`) (`self.combinedOffset`)) false true)))
    (set `self.combinedOffset` (+ (`self.lowOffset`) (`self.combinedOffset`)))))

(fn `UserConstructionScript`)